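; BP_RaccoonExpress is a gameplay Blueprint that manages a draining gas supply for the Raccoon Express.
; BeginPlay sets game-only input, fills gas to its maximum and adds the WBP_HUD widget to the viewport.
; Tick drains one gas unit per second, printing the rounded-up amount, or a "Dead Raccoon" debug message at empty.
; AddGas refills the supply, clamped between zero and the maximum.
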(event `self.ReceiveBeginPlay`
  (`WidgetBlueprintLibrary.SetInputMode_GameOnly` (`GameplayStatics.GetPlayerController` 0))
  (set `self.GasCurrent` (`self.GasMax`))
  (bind _returnvalue (`|CreateWidget` "/Game/Blueprints/WBP_HUD.WBP_HUD_C"))
  (`UserWidget.AddToViewport` _returnvalue 0))

(event `self.ReceiveTick`
  (params (DeltaSeconds :type "Float (single-precision)"))
  (bind _output_get (set `self.GasCurrent` (`KismetMathLibrary.FClamp` (- (`self.GasCurrent`) DeltaSeconds) 0.0 (`self.GasMax`))))
  (if (== _output_get 0.0)
    (`KismetSystemLibrary.PrintString` "Dead Raccoon" true false (struct :`R` 1.0 :`B` 0.057999 :`A` 1.0) 2.0 "asdaadadsadadawfasf")
    (else
      (`KismetSystemLibrary.PrintString` (`KismetStringLibrary.Concat_StrStr` "Gas: " (`KismetStringLibrary.Conv_IntToString` (`KismetMathLibrary.FCeil` _output_get))) true false (struct :`G` 0.66 :`B` 1.0 :`A` 1.0) 2.0 "asdaadadsadadawfasf"))))

(fn `AddGas`
  (params (AddAmount :type "Float (double-precision)"))
  (set `self.GasCurrent` (`KismetMathLibrary.FClamp` (+ AddAmount (`self.GasCurrent`)) 0.0 (`self.GasMax`))))

(fn `UserConstructionScript`)